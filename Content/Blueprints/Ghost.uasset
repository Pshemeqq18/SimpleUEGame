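; Ghost enemy character that drifts along negative X and costs the player health when it hits a platform.
; Movement comes from LaunchCharacter at spawn and again on Tick whenever velocity is zero, with the capsule ignoring the MainCharacter while moving.
; Hits are classified by display-name prefix: bullets drain HP until it explodes, while platforms trigger a big explosion and GameOverManager.SubstractHealth.
; Both endings destroy the actor after a short delay.
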(event EventBeginPlay
  (Pawn|SpawnDefaultController)
  (Character|LaunchCharacter "-30.000000,0.000000,0.000000" false false)
  (Variables|Default|SetHP 100)
  (bind _returnvalue (Actor|GetActorOfClass "/Game/Blueprints/GameOverManager.GameOverManager_C"))
  (Variables|Default|SetGameOverManager _returnvalue)
  (bind _returnvalue_2 (Actor|GetActorOfClass "/Game/Blueprints/MainCharacter.MainCharacter_C"))
  (bind _output_get (Variables|Default|SetMainCharacter _returnvalue_2))
  (Collision|IgnoreActorwhenMoving (Variables|Collision|GetCapsuleComponent) _output_get true))

(event EventTick
  (params (DeltaSeconds :type Float%20%28single-precision%29))
  (if (== (Math|Vector|VectorLength (Transformation|GetVelocity)) 0.0)
    (Character|LaunchCharacter "-30.000000,0.000000,0.000000" false false)))

(event Collision|EventHit
  (params (MyComp :type Primitive%20Component%20Object%20Reference) (Other :type Actor%20Object%20Reference) (OtherComp :type Primitive%20Component%20Object%20Reference) (bSelfMoved :type Boolean) (HitLocation :type Vector :default "0, 0, 0") (HitNormal :type Vector :default "0, 0, 0") (NormalImpulse :type Vector :default "0, 0, 0") (Hit :type Hit%20Result%20Structure%20%28by%20ref%29))
  (bind _returnvalue (Utilities|GetDisplayName Other))
  (if (not (Variables|Default|GetOver))
    (if (Utilities|String|StartsWith _returnvalue "Bullet")
      (bind _output_get (Variables|Default|SetHP (- (Variables|Default|GetHP) 15)))
      (if (not (> _output_get 0))
        (Sprite|SetFlipbook (Variables|Default|GetSprite) "/Game/Sprites/Super_Grotto_Escape_Files/Fx/Sprites/Explosion/explosion.explosion")
        (Utilities|FlowControl|Delay 0.2)
        (Actor|DestroyActor))
      (elif (Utilities|String|StartsWith _returnvalue "Platform")
        (Variables|Default|SetOver true)
        (Sprite|SetFlipbook (Variables|Default|GetSprite) "/Game/Sprites/Super_Grotto_Escape_Files/Fx/Sprites/Big-Explosion/big-explosion.big-explosion")
        (Default|SubstractHealth (Variables|Default|GetGameOverManager))
        (Utilities|FlowControl|Delay 1.5)
        (Actor|DestroyActor)))))

(fn ConstructionScript)