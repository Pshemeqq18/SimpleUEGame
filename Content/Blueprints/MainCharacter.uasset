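; Player character for a Paper2D side-scroller that runs along X, jumps and shoots.
; Move input flips the sprite's X scale, which sets the side a Bullet spawns on and its direction.
; Shooting sets a brief IsShooting lock that also overrides the velocity-driven idle, run, jump and fall flipbooks chosen each Tick.
; Tick also snaps any Y drift back to zero, resetting rotation and scale.
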(event Custom|Handle%20Animations
  (bind _charactermovement (Variables|Character|GetCharacterMovement))
  (bind _velocity (Variables|/Script/Engine.MovementComponent|GetVelocity _charactermovement))
  (bind (_x _y _z) (Math|Vector|BreakVector _velocity))
  (if (Variables|Default|GetIsShooting)
    (Sprite|SetFlipbook (Variables|Default|GetSprite) "/Game/Sprites/Super_Grotto_Escape_Files/Characters/Player/sprites/Player-run-shoot/player-run-shoott.player-run-shoott")
    (elif (!= _z 0.0)
      (if (> _z 0.0)
        (Sprite|SetFlipbook (Variables|Default|GetSprite) "/Game/Sprites/Super_Grotto_Escape_Files/Characters/Player/sprites/Player-jump/player-jump.player-jump")
        (else
          (Sprite|SetFlipbook (Variables|Default|GetSprite) "/Game/Sprites/Super_Grotto_Escape_Files/Characters/Player/sprites/Player-jump/player-falling.player-falling")))
      (else
        (Sprite|SetFlipbook (Variables|Default|GetSprite) (select (!= _x 0.0) "/Game/Sprites/Super_Grotto_Escape_Files/Characters/Player/sprites/player-run/player-run.player-run" "/Game/Sprites/Super_Grotto_Escape_Files/Characters/Player/sprites/Player-idle/player-idle.player-idle"))))))

(event EventBeginPlay
  (Variables|Default|SetIsShooting false))

(event Collision|EventActorBeginOverlap
  (params (OtherActor :type Actor%20Object%20Reference)))

(event EventTick
  (params (DeltaSeconds :type Float%20%28single-precision%29))
  (bind _returnvalue (Transformation|GetActorTransform))
  (bind _location (Math|Transform|BreakTransform _returnvalue))
  (bind (_x _y _z) (Math|Vector|BreakVector _location))
  (CallFunction|HandleAnimations)
  (if (!= _y 0.0)
    (Transformation|SetActorTransform (Math|Transform|MakeTransform (Math|Vector|MakeVector _x 0.0 _z) "0, 0, 0" "0.800000,0.800000,0.800000"))))

(event Input|ActionEvents|InputActionJump
  (params (Key :type Key%20Structure :default "None"))
  (:Pressed
    (Character|Jump)))

(event Input|ActionEvents|InputActionShoot
  (params (Key :type Key%20Structure :default "None"))
  (bind _returnvalue (Transformation|GetActorTransform))
  (bind _sprite (Variables|Default|GetSprite))
  (bind (_location _rotation _scale) (Math|Transform|BreakTransform _returnvalue))
  (bind _returnvalue_2 (Transformation|GetWorldScale _sprite))
  (bind (_x _y _z) (Math|Vector|BreakVector _location))
  (bind _x_2 (Math|Vector|BreakVector _returnvalue_2))
  (:Pressed
    (if (not (Variables|Default|GetIsShooting))
      (Variables|Default|SetIsShooting true)
      (bind _output_get (Variables|Default|SetIsFacingRight (> _x_2 0.0)))
      (Game|SpawnActorfromClass "/Game/Blueprints/Bullet.Bullet_C" (Math|Transform|MakeTransform (Math|Vector|MakeVector (+ _x (* _x_2 18.0)) _y _z) _rotation _scale) "Undefined" "MultiplyWithRoot" 0 _output_get 0)
      (Utilities|FlowControl|Delay 0.1)
      (Variables|Default|SetIsShooting false))))

(event Input|AxisEvents|InputAxisMoveLeft/Right
  (params (AxisValue :type Float%20%28single-precision%29))
  (Pawn|Input|AddMovementInput "1.000000,0.000000,0.000000" AxisValue false))

(event Input|AxisEvents|InputAxisMoveLeft/Right
  (params (AxisValue :type Float%20%28single-precision%29))
  (switch int (+ (Math|Float|Truncate AxisValue) 1)
    (:0
      (Transformation|SetRelativeScale3D (Variables|Default|GetSprite) "-1.000000,1.000000,1.000000"))
    (:2
      (Transformation|SetRelativeScale3D (Variables|Default|GetSprite) "1.000000,1.000000,1.000000"))))

(fn ConstructionScript)