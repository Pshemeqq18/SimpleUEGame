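; Spawn manager actor that repeatedly spawns an actor, presumably a ghost, at one of three vertical lanes.
; BeginPlay starts SpawnGhost, a custom event that waits on a short Delay, spawns, then calls itself to loop indefinitely.
; Each spawn uses a fixed X and Y with a random, evenly spaced Z offset, and is skipped if it would collide.
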(event Custom|SpawnGhost
  (Utilities|FlowControl|Delay 2.0)
  (Game|SpawnActorfromClass "/Game/Blueprints/Ghost.Ghost_C" (Math|Transform|MakeTransform (Math|Vector|MakeVector 2e+02 0.0 (Math|Conversions|ToFloat(Integer) (+ (* (Math|Random|RandomIntegerinRange -1 1) 47) -17)))) "DontSpawnIfColliding" "MultiplyWithRoot" 0 0)
  (CallFunction|SpawnGhost))

(event EventBeginPlay
  (CallFunction|SpawnGhost))

(event Collision|EventActorBeginOverlap
  (params (OtherActor :type Actor%20Object%20Reference)))

(event EventTick
  (params (DeltaSeconds :type Float%20%28single-precision%29)))

(fn ConstructionScript)