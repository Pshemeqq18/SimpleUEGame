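; Bullet is a character-based projectile with a flipbook sprite, apparently fired by the player.
; On BeginPlay it spawns a default controller and launches itself along world X, with the IsTurnedRight flag choosing the direction.
; On any hit it stops moving, disables collision, switches to the shot-hit flipbook and destroys itself after a short delay.
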(event EventBeginPlay
  (Pawn|SpawnDefaultController)
  (if (Variables|Default|GetIsTurnedRight)
    (Character|LaunchCharacter "400.000000,0.000000,0.000000" false false)
    (else
      (Character|LaunchCharacter "-400.000000,0.000000,0.000000" false false))))

(event EventTick
  (params (DeltaSeconds :type Float%20%28single-precision%29)))

(event Collision|EventHit
  (params (MyComp :type Primitive%20Component%20Object%20Reference) (Other :type Actor%20Object%20Reference) (OtherComp :type Primitive%20Component%20Object%20Reference) (bSelfMoved :type Boolean) (HitLocation :type Vector :default "0, 0, 0") (HitNormal :type Vector :default "0, 0, 0") (NormalImpulse :type Vector :default "0, 0, 0") (Hit :type Hit%20Result%20Structure%20%28by%20ref%29))
  (Components|Movement|StopMovementImmediately (Variables|Character|GetCharacterMovement))
  (Collision|SetActorEnableCollision false)
  (Sprite|SetFlipbook (Variables|Default|GetSprite) "/Game/Sprites/Super_Grotto_Escape_Files/Fx/Sprites/Player-shoot-hit/player-shoot-hit.player-shoot-hit")
  (Utilities|FlowControl|Delay 0.2)
  (Actor|DestroyActor))

(fn ConstructionScript)